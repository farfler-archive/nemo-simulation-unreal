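; BP_Wheelchair is a player-controlled wheelchair driven by movement and rotation input.
; The move axis offsets it along its local forward axis, scaled by MoveSpeed, without sweep, and the rotate axis yaws it by the raw axis value.
; ResetWheelchair sets its rotation using only the current yaw, righting it.
; Freecam spawns a BP_DebugPawn at the wheelchair's transform and has the first player controller possess it.
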(event EventBeginPlay)

(event Collision|EventActorBeginOverlap
  (params (OtherActor :type Actor%20Object%20Reference)))

(event EventTick
  (params (DeltaSeconds :type Float%20%28single-precision%29)))

(event Input|ActionEvents|InputActionFreecam
  (params (Key :type Key%20Structure :default "None"))
  (:Pressed
    (bind _returnvalue (Game|SpawnActorfromClass "/Game/Blueprints/BP_DebugPawn.BP_DebugPawn_C" (Transformation|GetActorTransform) "Undefined" "MultiplyWithRoot" 0 0))
    (Pawn|Possess (Game|GetPlayerController 0) _returnvalue)))

(event Input|ActionEvents|InputActionResetWheelchair
  (params (Key :type Key%20Structure :default "None"))
  (:Pressed
    (Transformation|SetActorRotation (Math|Rotator|MakeRotator 0.0 0.0 (.yaw (Transformation|GetActorRotation))))))

(event Input|AxisEvents|InputAxisMoveHorizontal
  (params (AxisValue :type Float%20%28single-precision%29))
  (Transformation|AddActorLocalOffset (* (Class|KismetMathLibrary|VectorForward) (* AxisValue (Variables|Default|GetMoveSpeed))) false false))

(event Input|AxisEvents|InputAxisRotate
  (params (AxisValue :type Float%20%28single-precision%29))
  (Transformation|AddActorLocalRotation (Math|Rotator|MakeRotator 0.0 0.0 AxisValue) false false))

(fn ConstructionScript)